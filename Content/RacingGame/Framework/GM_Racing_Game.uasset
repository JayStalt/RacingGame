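; Racing game mode that runs a countdown, then a time limit, and prints a win or lose message.
; On BeginPlay it binds events to every EP_Checkpoint, separating the finish line from timed checkpoints.
; Timer expiry triggers a loss, while Win clears the timer.
; Checkpoint time is added to the StartTimerDuration variable only, without resetting the running timer.
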(event Custom|Game%20End
  (params (Win :type Boolean))
  (Development|PrintString (Utilities|String|SelectString "You win!" "You Lose!" Win)))

(event Custom|Game%20Start
  (Development|PrintString "Game has Started")
  (bind _returnvalue (Utilities|Time|SetTimerbyEvent (delegate Custom|Lose?%20OutofTime) (Variables|Default|GetStartTimer%20Duration)))
  (Variables|Default|SetTimeRemainingTimer _returnvalue))

(event Custom|Start%20Countdown
  (Development|PrintString "Start Countdown")
  (Utilities|FlowControl|Delay (Variables|Default|GetStartCountdownDuration))
  (CallFunction|GameStart))

(event Custom|Lose?%20OutofTime
  (CallFunction|GameEnd false))

(event Custom|Win
  (Utilities|Time|ClearandInvalidateTimerbyHandle (Variables|Default|GetTimeRemainingTimer))
  (CallFunction|GameEnd true))

(event Custom|CrossedCheckpoint
  (params (Time%20to%20Add :type Integer))
  (CallFunction|AddTimetoTimer Time%20to%20Add))

(event EventBeginPlay
  (Utilities|FlowControl|Sequence
    (:then_0
      (bind _outactors (Actor|GetAllActorsOfClass "/Game/RacingGame/CheckPoints/EP_Checkpoint.EP_Checkpoint_C"))
      (for _array_element _outactors
        (if (Variables|/Game/RacingGame/CheckPoints/EP_Checkpoint.EP_Checkpoint_C|GetIsFinishLine _array_element)
          (EventDispatchers|BindEventtoOnCheckPointCrossed _array_element (EventDispatchers|CreateEvent :!event Custom|Win))
          (else
            (EventDispatchers|BindEventtoOnCheckPointCrossedwithTime _array_element (EventDispatchers|CreateEvent :!event Custom|CrossedCheckpoint))))))
    (:then_1
      (CallFunction|StartCountdown))))

(fn ConstructionScript)

(fn AddTimetoTimer
  (params (TimeToAdd :type Integer))
  (Variables|Default|SetStartTimer%20Duration (+ (Variables|Default|GetStartTimer%20Duration) TimeToAdd)))